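; BP_HideBox is a possessable hiding box that the player character can enter and leave.
; Its Box overlap flags the player as in range to possess and passes it a reference to the box, clearing the flag on exit.
; While possessed, the box forwards Turn and LookUp to controller rotation.
; Pressing E makes the stored character's capsule and children visible and re-possesses that character.
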(event OnComponentBeginOverlap(Box)
  (params (OverlappedComponent :type Primitive%20Component%20Object%20Reference) (OtherActor :type Actor%20Object%20Reference) (OtherComp :type Primitive%20Component%20Object%20Reference) (OtherBodyIndex :type Integer) (bFromSweep :type Boolean) (SweepResult :type Hit%20Result%20Structure%20%28by%20ref%29))
  (bind _asbp_player_character (Utilities|Casting|CastToBP_PlayerCharacter OtherActor))
  (Variables|/Game/Core/Character/BP_PlayerCharacter.BP_PlayerCharacter_C|SetPlayerIsInRangeToPossess _asbp_player_character true)
  (Variables|/Game/Core/Character/BP_PlayerCharacter.BP_PlayerCharacter_C|SetPocessBoxActor _asbp_player_character self)
  (Variables|Default|SetBp_PlayerCharacter _asbp_player_character))

(event OnComponentEndOverlap(Box)
  (params (OverlappedComponent :type Primitive%20Component%20Object%20Reference) (OtherActor :type Actor%20Object%20Reference) (OtherComp :type Primitive%20Component%20Object%20Reference) (OtherBodyIndex :type Integer))
  (bind _asbp_player_character (Utilities|Casting|CastToBP_PlayerCharacter OtherActor))
  (Variables|/Game/Core/Character/BP_PlayerCharacter.BP_PlayerCharacter_C|SetPlayerIsInRangeToPossess _asbp_player_character false))

(event Input|AxisEvents|InputAxisTurn
  (params (AxisValue :type Float%20%28single-precision%29))
  (Pawn|Input|AddControllerYawInput AxisValue))

(event Input|AxisEvents|InputAxisLookUp
  (params (AxisValue :type Float%20%28single-precision%29))
  (Pawn|Input|AddControllerPitchInput AxisValue))

(event Input|KeyboardEvents|E
  (params (Key :type Key%20Structure :default "None"))
  (:Pressed
    (Rendering|SetVisibility (Variables|/Script/Engine.Character|GetCapsuleComponent (Variables|Default|GetBp_PlayerCharacter)) true true)
    (Pawn|Possess (Game|GetPlayerController 0) (Variables|Default|GetBp_PlayerCharacter))))

(fn ConstructionScript)